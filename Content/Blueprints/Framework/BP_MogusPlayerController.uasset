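; Player controller for a traitor-style multiplayer game, handling ability use, traitor-to-boss transformation, pause menu and traitor kill reporting.
; The server runs the player state's ability from DT_AbilityStats as timed cone-trace damage ticks with a fixed cooldown, relaying sound and VFX through BP_Character.
; Replicated traitor state triggers owner-side UI, and deaths prompt game-state condition checks.
; Picked-class initialization on BeginPlay is disabled.
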(event Custom|Death
  (params (Killer :type Controller%20Object%20Reference) (Actor :type Actor%20Object%20Reference))
  (CallFunction|TryReportTraitorKill Killer))

(event Custom|Server_TryTransform
  ;[0.07187 0.004718 0.007722] Traitor/Boss
  (if (Variables|Default|GetIsTraitor)
    (if (not (Variables|Default|GetIsBoss))
      (Variables|Default|SetIsBoss true)
      (bind _asbp_character (Utilities|Casting|CastToBP_Character (Pawn|GetControlledPawn)))
      (Default|TranceformtoBoss _asbp_character))))

(event Custom|Owner_InitializeBoss
  ;[0.07187 0.004718 0.007722] Traitor/Boss
  ;;[0.131 0.03631 0.2969] owning client reaction
  (if (Pawn|IsLocalPlayerController)
    (if (Variables|Default|GetIsBoss)
      (Development|PrintString "You are now a boss" true true "(R=1.000000,G=0.030432,B=0.000000,A=1.000000)")
      (else
        (Development|PrintString "You are no longer a boss" true true "(R=1.000000,G=0.030432,B=0.000000,A=1.000000)")))))

(event Custom|Server_TryUseAbility
  (bind _returnvalue (Pawn|GetControlledPawn))
  ;[0.9802 0.5544 0.7057] Abilities
  (if (and (not (Variables|/Game/Blueprints/Framework/BP_MogusPlayerState.BP_MogusPlayerState_C|GetIsDead (Variables|Default|GetMogusPlayerState))) (Variables|Ability|GetCanUseAbility))
    (bind _mogusplayerstate (Variables|Default|GetMogusPlayerState)
      (:then
        (CallFunction|PlaySound (CallFunction|GetAbilitySound (Variables|/Game/Blueprints/Framework/BP_MogusPlayerState.BP_MogusPlayerState_C|GetPlayerAbility _mogusplayerstate)) false)
        (bind _asbp_character (Utilities|Casting|CastToBP_Character (Pawn|GetControlledPawn)))
        (Default|MulticastPlayAbilityVFX _asbp_character (Variables|/Game/Blueprints/Framework/BP_MogusPlayerState.BP_MogusPlayerState_C|GetPlayerAbility _mogusplayerstate))
        (bind _asbp_mogus_game_state (Utilities|Casting|CastToBP_MogusGameState (Game|GetGameState))
          (:then
            (Default|ServerReportAbilityUse _asbp_mogus_game_state (Variables|/Game/Blueprints/Framework/BP_MogusPlayerState.BP_MogusPlayerState_C|GetPlayerAbility _mogusplayerstate)))
          (:CastFailed
            _))
        (bind _returnvalue_2 (Utilities|GetDataTableRow "/Game/Blueprints/Framework/Abilities/DT_AbilityStats.DT_AbilityStats" (Utilities|String|StringToName (Utilities|String|EnumtoString (Variables|/Game/Blueprints/Framework/BP_MogusPlayerState.BP_MogusPlayerState_C|GetPlayerAbility _mogusplayerstate))))
          (:then
            (bind _output_get (Variables|Ability|SetAbilityStats _returnvalue_2))
            (Variables|Ability|SetCanUseAbility false)
            (Utilities|FlowControl|Sequence
              (:then_0
                (Variables|Default|Seti 0.0)
                (if (< (Variables|Default|Geti) (.DurationSec (Utilities|Struct|BreakS_AbilityStats _output_get))) :!label _label
                  (Variables|Default|Seti (+ (Variables|Default|Geti) (.DelayBetweenHitsSec (Utilities|Struct|BreakS_AbilityStats _output_get))))
                  (bind _foundactors (CallFunction|ConeTrace self (Transformation|GetActorLocation _returnvalue) (Transformation|GetActorForwardVector _returnvalue) (.RayLength (Utilities|Struct|BreakS_AbilityStats _output_get)) (.EffectRadius (Utilities|Struct|BreakS_AbilityStats _output_get)) (Math|Conversions|ToLinearColor(Color) (.Color (Utilities|Struct|BreakS_AbilityStats _output_get))) (Utilities|Array|MakeArray "ObjectTypeQuery3") (Utilities|Array|MakeArray (Pawn|GetControlledPawn))))
                  (for _array_element _foundactors
                    (if (Utilities|IsValid _array_element)
                      (Game|Damage|ApplyDamage _array_element (.DamagePerSecond (Utilities|Struct|BreakS_AbilityStats _output_get)) self (Pawn|GetControlledPawn) (.DamageTypeClass (Utilities|Struct|BreakS_AbilityStats _output_get)))
                      (Rendering|Decal|SpawnDecalatLocation "/Game/Maps/LevelPrototyping/Materials/MI_Solid_Blue.MI_Solid_Blue" "30.000000,30.000000,30.000000" (Transformation|GetActorLocation _array_element) "-90.000000,0.000000,0.000000" 1.0)))
                  (Utilities|FlowControl|Delay (.DelayBetweenHitsSec (Utilities|Struct|BreakS_AbilityStats _output_get)))
                  (goto _label)))
              (:then_1
                ;;[0.05937 0.02525 0.01872] crude cooldown
                (Utilities|FlowControl|Delay 6.0)
                (Variables|Ability|SetCanUseAbility true))))))
      (:else))
    (else
      (Development|PrintString "Server: Can't use ability"))))

(event Custom|Owner_InitializeAbility
  ;[0.9802 0.5544 0.7057] Abilities
  (if (Pawn|IsLocalPlayerController)
    (bind _returnvalue (UserInterface|CreateWidget "/Game/UI/WBP_AbilityUI.WBP_AbilityUI_C" self))
    (UserInterface|Viewport|AddtoViewport _returnvalue 1)
    (CallFunction|PlaySound "/Game/Sounds/transform1_Cue.transform1_Cue" true)))

(event Custom|InitCharacterClass
  (bind _asbp_online_game_instance (Utilities|Casting|CastToBP_OnlineGameInstance (Game|GetGameInstance))
    (:then
      (bind _output_get (Variables|Default|SetChar%20Class (Default|GetCharacterClass _asbp_online_game_instance)))
      (Development|PrintString (Utilities|String|Append "set initCharClass to " (Utilities|GetClassDisplayName _output_get))))
    (:CastFailed
      (Development|PrintString "initCharClass failed"))))

(event Custom|InitPickedClass
  (if (Pawn|IsLocalPlayerController)
    (bind _asbp_online_game_instance (Utilities|Casting|CastToBP_OnlineGameInstance (Game|GetGameInstance)))
    (bind _asbp_mogus_player_state (Utilities|Casting|CastToBP_MogusPlayerState (Variables|GetPlayerState)))
    (Default|ServerSetClass _asbp_mogus_player_state (Variables|/Game/Blueprints/Framework/BP_OnlineGameInstance.BP_OnlineGameInstance_C|GetPickedClass _asbp_online_game_instance))))

(event Custom|Owner_InitializeTraitor
  ;[0.07187 0.004718 0.007722] Traitor/Boss
  ;;[0.131 0.03631 0.2969] owning client reaction
  (if (Pawn|IsLocalPlayerController)
    (Development|PrintString "You feel a sudden urge to kill your mates" true true "(R=1.000000,G=0.030432,B=0.000000,A=1.000000)" 1e+01)
    (bind _returnvalue (UserInterface|CreateWidget "/Game/UI/WBP_TraitorUI.WBP_TraitorUI_C" self))
    (UserInterface|Viewport|AddtoViewport _returnvalue 1)))

(event EventBeginPlay
  (CallFunction|InitPickedClass)
  (Input|SetInputModeGameOnly self false)
  (Utilities|FlowControl|Delay 1.0)
  (bind _asbp_mogus_player_state (Utilities|Casting|CastToBP_MogusPlayerState (Variables|GetPlayerState))
    (:then
      (bind _output_get (Variables|Default|SetMogusPlayerState _asbp_mogus_player_state))
      (EventDispatchers|AssignOnAbilityPicked _output_get (EventDispatchers|CreateEvent :!event Custom|Owner_InitializeAbility)))
    (:CastFailed
      (Development|PrintString "couldn't find MogusPlayerState"))))

(event Input|ActionEvents|InputActionUseAbility
  (params (Key :type Key%20Structure :default "None"))
  ;[0.9802 0.5544 0.7057] Abilities
  (:Pressed
    (if (Pawn|IsLocalPlayerController)
      (if (Variables|Ability|GetCanUseAbility)
        (CallFunction|ServerTryUseAbility)
        (else
          (Development|PrintString "Can't use ability")
          (CallFunction|PlaySound "/Game/Sounds/Abilities/ability_cooldown_Cue.ability_cooldown_Cue" true))))))

(event Input|KeyboardEvents|T
  (params (Key :type Key%20Structure :default "None"))
  ;[0.07187 0.004718 0.007722] Traitor/Boss
  (:Pressed
    (if (Variables|Default|GetIsTraitor)
      (CallFunction|ServerTryTransform) ; todo cooldwn
    )))

(event Input|KeyboardEvents|Escape
  (params (Key :type Key%20Structure :default "None"))
  (:Pressed
    (if (Pawn|IsLocalPlayerController)
      (CallFunction|TogglePauseMenu))))

(fn ConstructionScript)

(fn OnRepIsTraitor
  (if (Variables|Default|GetIsTraitor)
    (CallFunction|OwnerInitializeTraitor)))

(fn OnRepIsBoss
  (Development|PrintString (Utilities|String|Append (PlayerState|GetPlayerName (Variables|GetPlayerState)) " isBoss=" (Utilities|String|ToString(Boolean) (Variables|Default|GetIsBoss)))))

(fn TogglePauseMenu
  (Variables|Default|GetPauseMenu
    (:then
      (Widget|SetVisibility (Variables|Default|GetPauseMenu) "Collapsed")
      (Widget|RemovefromParent (Variables|Default|GetPauseMenu))
      (Variables|Default|SetPauseMenu 0)
      (Input|SetInputModeGameOnly self false)
      (Variables|Default|SetbShowMouseCursor false)
      (Development|PrintString "Pause menu off"))
    (:else
      (bind _returnvalue (UserInterface|CreateWidget "/Game/UI/WBP_PauseMenu.WBP_PauseMenu_C" (Game|GetPlayerController 0)))
      (bind _output_get (Variables|Default|SetPauseMenu _returnvalue))
      (UserInterface|Viewport|AddtoViewport _output_get 10)
      (Variables|/Script/UMG.Widget|SetVisibility (Variables|Default|GetPauseMenu) "Visible")
      (Input|SetInputModeUIOnly self (Variables|Default|GetPauseMenu) "LockInFullscreen" false)
      (Variables|Default|SetbShowMouseCursor true)
      (Development|PrintString "Pause menu on"))))

(fn OnRepCanUseAbility
  (if (Variables|Ability|GetCanUseAbility)
    (Development|PrintString "Can use ability")))

(fn PlaySound
  (params (Sound :type Sound%20Base%20Object%20Reference) (Local :type Boolean))
  (bind _asbp_character (Utilities|Casting|CastToBP_Character (Pawn|GetControlledPawn)))
  (if Local
    (Default|PlayLocalSound _asbp_character Sound)
    (else
      (Default|MulticastPlaySound _asbp_character Sound false))))

(fn GetAbilitySound
  (params (Ability :type E_PlayerAbility%20Enum :default "NewEnumerator0"))
  (switch Utilities|FlowControl|Switch|SwitchonE_PlayerAbility Ability
    (:NewEnumerator0
      (LocalVariables|SetFoundSound "/Game/Sounds/Abilities/ability_kek_Cue.ability_kek_Cue"))
    (:NewEnumerator1
      (LocalVariables|SetFoundSound "/Game/Sounds/Abilities/ability_fire_Cue.ability_fire_Cue"))
    (:NewEnumerator2
      (LocalVariables|SetFoundSound "/Game/Sounds/Abilities/ability_water_Cue.ability_water_Cue"))
    (:NewEnumerator3
      (LocalVariables|SetFoundSound "/Game/Sounds/Abilities/ability_earth_Cue.ability_earth_Cue"))
    (:NewEnumerator4
      (LocalVariables|SetFoundSound "/Game/Sounds/Abilities/ability_air_Cue.ability_air_Cue"))
    (:NewEnumerator5
      (LocalVariables|SetFoundSound "/Game/Sounds/Abilities/ability_love_Cue.ability_love_Cue")))
  (return (LocalVariables|GetFoundSound)))

(fn PlayAbilityVFX
  (params (Ability :type E_PlayerAbility%20Enum :default "NewEnumerator0"))
  (bind _returnvalue (Utilities|GetDataTableRow "/Game/Blueprints/Framework/Abilities/DT_AbilityStats.DT_AbilityStats" (Utilities|String|StringToName (Utilities|String|EnumtoString Ability)))
    (:then
      (LocalVariables|SetLength (.raylength _returnvalue))
      (LocalVariables|SetWidth (.effectradius _returnvalue))
      (LocalVariables|SetColor (.color _returnvalue))
      (LocalVariables|SetDuration (.durationsec _returnvalue))
      (bind _asbp_character (Utilities|Casting|CastToBP_Character (Pawn|GetControlledPawn)))
      (LocalVariables|SetAttachedSystem (Variables|/Game/Blueprints/Characters/BP_Character.BP_Character_C|GetNS_Attached _asbp_character))
      (switch Utilities|FlowControl|Switch|SwitchonE_PlayerAbility Ability
        (:NewEnumerator1
          (Class|NiagaraComponent|SetAsset (LocalVariables|GetAttachedSystem) 0 true)
          (Class|NiagaraComponent|SetAsset (LocalVariables|GetAttachedSystem) "/Game/Wathammer/Asset/NiagaraFX/Weapons/Trace_Weapons/Flamethrower/NS_flametrower_parameter.NS_flametrower_parameter" true))
        (:NewEnumerator2
          (Niagara|SpawnSystematLocation "/Game/Wathammer/Asset/NiagaraFX/HeartFX/NS_Heart_atacked.NS_Heart_atacked" (Transformation|GetWorldLocation (LocalVariables|GetAttachedSystem)) (Math|Conversions|RotationFromXVector (Math|Vector|GetForwardVector (LocalVariables|GetAttachedSystem)))))
        (:NewEnumerator3
          (Niagara|SpawnSystematLocation "/Game/FX/my_fx_volnitsa/Effect05_earthSpikes/NS_EarthSpikesConeWave.NS_EarthSpikesConeWave" (Transformation|GetWorldLocation (Variables|/Script/Engine.Character|GetMesh _asbp_character)) (Math|Conversions|RotationFromXVector (Math|Vector|GetForwardVector (LocalVariables|GetAttachedSystem)))))
        (:NewEnumerator4
          (Niagara|SpawnSystematLocation "/Game/FX/AirVFX/NS_AirSmokeWave.NS_AirSmokeWave" (Transformation|GetWorldLocation (Variables|/Script/Engine.Character|GetMesh _asbp_character)) (Math|Conversions|RotationFromXVector (Math|Vector|GetForwardVector (LocalVariables|GetAttachedSystem)))))
        (:NewEnumerator5
          (Niagara|SpawnSystematLocation "/Game/Wathammer/Asset/NiagaraFX/Weapons/Impact_Weapons/PlasmaGun/NS_plasmagun_impact.NS_plasmagun_impact" (Transformation|GetWorldLocation (LocalVariables|GetAttachedSystem)) (Math|Conversions|RotationFromXVector (Math|Vector|GetForwardVector (LocalVariables|GetAttachedSystem)))))))))

(fn TryReportTraitorKill
  (params (Killer :type Controller%20Object%20Reference))
  (bind _asbp_mogus_game_state (Utilities|Casting|CastToBP_MogusGameState (Game|GetGameState)))
  (Default|ServerCheckAllConditions _asbp_mogus_game_state)
  (bind _asbp_mogus_player_controller (Utilities|Casting|CastToBP_MogusPlayerController Killer)
    (:then
      (if (Variables|BP_MogusPlayerController_C|GetIsTraitor _asbp_mogus_player_controller)
        (Default|ServerReportTraitorKill _asbp_mogus_game_state)
        (return)))
    (:CastFailed
      (return))))