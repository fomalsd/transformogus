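; Game state for the online Mogus game that picks one random player as the traitor.
; A server check scans every player state for an unchosen ability, printing names of those still missing, and triggers the pick once all have chosen.
; The pick runs once, guarded by a flag, and marks the chosen player's controller as traitor.
; On BeginPlay it also stops the menu music through the online game instance.
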(event Custom|Server_PickTraitor
  (if (Variables|ServerOnly|GetIsTraitorPicked)
    (Development|PrintString "Traitor already picked")
    (else
      (Variables|ServerOnly|SetIsTraitorPicked true)
      (bind _asbp_mogus_player_controller (Utilities|Casting|CastToBP_MogusPlayerController (Game|GetPlayerController (.OutItem (Utilities|Array|Random (Variables|Default|GetPlayerArray))))))
      (bind _output_get (Variables|ServerOnly|SetTraitor _asbp_mogus_player_controller))
      (Variables|/Game/Blueprints/Framework/BP_MogusPlayerController.BP_MogusPlayerController_C|SetIsTraitor _output_get true))))

(event Custom|Server_CheckPickTraitor
  (if (Variables|ServerOnly|GetIsTraitorPicked)
    (Development|PrintString "Traitor already picked")
    (else
      (Variables|ServerOnly|SetAllAbilitiesPicked true)
      (for _array_element (Variables|Default|GetPlayerArray)
        (bind _asbp_mogus_player_state (Utilities|Casting|CastToBP_MogusPlayerState _array_element))
        (if (Utilities|Enum|Equal(Enum) (Variables|/Game/Blueprints/Framework/BP_MogusPlayerState.BP_MogusPlayerState_C|GetPlayerAbility _asbp_mogus_player_state) "NewEnumerator0")
          (Variables|ServerOnly|SetAllAbilitiesPicked false)
          (Development|PrintString (Utilities|String|Append (PlayerState|GetPlayerName _asbp_mogus_player_state) " didn't pick ability yet"))))
      (if (Variables|ServerOnly|GetAllAbilitiesPicked)
        (CallFunction|ServerPickTraitor)))))

(event EventBeginPlay
  (bind _asbp_online_game_instance (Utilities|Casting|CastToBP_OnlineGameInstance (Game|GetGameInstance)))
  (Default|StopMenuMusic _asbp_online_game_instance))

(fn ConstructionScript)