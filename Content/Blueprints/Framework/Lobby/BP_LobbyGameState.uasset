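; Lobby game state that runs the ready check and countdown before the match travels to the main map.
; When every player state reports ready, the server sets the replicated counting flag, whose RepNotify broadcasts countdown start, then fires a completion dispatcher after a delay.
; A delayed Tick decrements the remaining seconds on authority.
; The start-game event logs each player's picked class and server-travels; BeginPlay binds a completion handler on authority.
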(event Custom|Server_StartGame
  (for _array_element (Variables|Default|GetPlayerArray)
    (bind _asbp_lobby_player_state (Utilities|Casting|CastToBP_LobbyPlayerState _array_element))
    (Development|PrintText (Utilities|Text|FormatText "Preparing to travel with {playerName} as a {playerClass}" (PlayerState|GetPlayerName _asbp_lobby_player_state) (Utilities|String|EnumtoString (Variables|/Game/Blueprints/Framework/Lobby/BP_LobbyPlayerState.BP_LobbyPlayerState_C|GetPickedClass _asbp_lobby_player_state)))))
  (Class|AdvancedSessionsLibrary|ServerTravel "/Game/Maps/MainMap_persistent" false false))

(event Custom|Server_CheckStartCountdown
  (Development|PrintString "Started server countdown")
  (if (not (Variables|Default|GetIsCounting))
    (Variables|Default|SetAllReady true)
    (for _array_element (Variables|Default|GetPlayerArray)
      (bind _asbp_lobby_player_state (Utilities|Casting|CastToBP_LobbyPlayerState _array_element))
      (if (Variables|/Game/Blueprints/Framework/Lobby/BP_LobbyPlayerState.BP_LobbyPlayerState_C|GetIsReady _asbp_lobby_player_state)
        (Development|PrintString (Utilities|String|Append (PlayerState|GetPlayerName _asbp_lobby_player_state) " is ready"))
        (else
          (Variables|Default|SetAllReady false)
          (Development|PrintString (Utilities|String|Append (PlayerState|GetPlayerName _asbp_lobby_player_state) " isn't ready yet")))))
    (if (Variables|Default|GetAllReady)
      (Variables|Default|SetIsCounting true)
      (Variables|Default|SetSecondsRemaining (Variables|Default|GetCountdownSeconds))
      (Utilities|FlowControl|Delay (Variables|Default|GetCountdownSeconds))
      (Default|CallOnCountdownComplete)
      (else
        (Development|PrintString "Not everyone is ready yet")))))

(event EventTick
  (params (DeltaSeconds :type Float%20%28single-precision%29))
  (if (Math|Boolean|ANDBoolean (Variables|Default|GetIsCounting) (> (Variables|Default|GetSecondsRemaining) 0.0) (Ability|HasAuthority))
    (Utilities|FlowControl|Delay 1.0)
    (Math|Float|DecrementFloat (Variables|Default|GetSecondsRemaining))))

(event EventBeginPlay
  (Networking|SwitchHasAuthority
    (:Authority
      (EventDispatchers|BindEventtoOnCountdownComplete (EventDispatchers|CreateEvent :!event Custom|Server_StartGame)))))

(fn ConstructionScript)

(fn OnRepIsCounting
  (if (Variables|Default|GetIsCounting)
    (Default|CallOnCountdownStart)))