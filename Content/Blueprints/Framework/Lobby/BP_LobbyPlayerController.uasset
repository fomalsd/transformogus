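; Lobby player controller that shows the host menu widget with the mouse cursor and handles character class switching.
; ChangeClassActor has the owner store the pick in the game instance, clears the pawn and its attached actors, then spawns and possesses the mapped class at the same transform.
; Owner and multicast events handle saving the class, destroying attachments and, after a short delay, adding a player-name text render to the new pawn.
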(event Custom|CreateMenus
  (bind _returnvalue (UserInterface|CreateWidget "/Game/UI/Lobby/WBP_LobbyHostMenu.WBP_LobbyHostMenu_C"))
  (bind _output_get (Variables|Default|SetLobbyMenu _returnvalue))
  (UserInterface|Viewport|AddtoViewport _output_get 0))

(event Custom|ChangeClassActor
  (params (NewClass :type E_PlayerClass%20Enum :default "NewEnumerator0"))
  (bind _returnvalue (Pawn|GetControlledPawn))
  (CallFunction|OwnerSetCharClass NewClass)
  (Variables|Default|SetTemp_Transform (Transformation|GetActorTransform _returnvalue))
  (bind _asbp_online_game_instance (Utilities|Casting|CastToBP_OnlineGameInstance (Game|GetGameInstance)))
  (for _array_element (Actor|GetAttachedActors _returnvalue true true)
    (CallFunction|MulticastDestroyGun _array_element))
  (Actor|DestroyActor _returnvalue)
  (bind _returnvalue_2 (Game|SpawnActorfromClass (.Value (Utilities|Map|Find (Variables|/Game/Blueprints/Framework/BP_OnlineGameInstance.BP_OnlineGameInstance_C|GetClassToCharacter _asbp_online_game_instance) NewClass)) (Variables|Default|GetTemp_Transform) "AlwaysSpawn" "MultiplyWithRoot" 0 0))
  (Pawn|Possess _returnvalue_2)
  (Utilities|FlowControl|Delay 0.2)
  (CallFunction|MulticastAddNameText))

(event Custom|Multicast_DestroyGun
  (params (Child :type Actor%20Object%20Reference))
  (if (Utilities|IsValid Child)
    (Actor|DestroyActor Child)))

(event Custom|Multicast_AddNameText
  (bind _returnvalue (Pawn|GetControlledPawn))
  (if (Utilities|IsValid _returnvalue)
    (bind _returnvalue_2 (Game|AddComponentbyClass _returnvalue "/Script/Engine.TextRenderComponent" false (Math|Conversions|ToTransform(Vector) "60.000000,0.000000,-50.000000")))
    (Rendering|Components|TextRender|SetHorizontalAlignment _returnvalue_2 "EHTA_Center")
    (Rendering|Components|TextRender|SetWorldSize _returnvalue_2 12.0)
    (Rendering|Components|TextRender|SetText _returnvalue_2 (Utilities|Text|ToText(String) (PlayerState|GetPlayerName (Variables|GetPlayerState))))))

(event Custom|Owner_SetCharClass
  (params (PlayerClass :type E_PlayerClass%20Enum :default "NewEnumerator0"))
  (Development|PrintString (Utilities|String|Append "Set picked character class to " (Utilities|String|EnumtoString PlayerClass)))
  (bind _asbp_online_game_instance (Utilities|Casting|CastToBP_OnlineGameInstance (Game|GetGameInstance)))
  (Variables|/Game/Blueprints/Framework/BP_OnlineGameInstance.BP_OnlineGameInstance_C|SetPickedClass _asbp_online_game_instance PlayerClass))

(event EventBeginPlay
  (CallFunction|CreateMenus)
  (Variables|Default|SetbShowMouseCursor true))

(fn ConstructionScript)