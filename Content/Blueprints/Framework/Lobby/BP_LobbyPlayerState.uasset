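; Lobby player state that tracks each player's picked class and ready status through RepNotify variables.
; Server_SetClass stores the class and records it by the player's unique ID in the game instance's ConnectionToClass map, while Server_SetReady marks the player ready.
; Both OnRep functions print debug messages, then on authority have the lobby player controller change the class actor or the lobby game state check the start countdown.
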(event Custom|Server_SetReady
  (Variables|Default|SetIsReady true))

(event Custom|Server_SetClass
  (params (PlayerClass :type E_PlayerClass%20Enum :default "NewEnumerator0"))
  (bind _output_get (Variables|Default|SetPickedClass PlayerClass))
  (bind _asbp_online_game_instance (Utilities|Casting|CastToBP_OnlineGameInstance (Game|GetGameInstance)))
  (Development|PrintText (Utilities|Text|FormatText "Server added pair {netid}/{class}" (PlayerState|GetPlayerName) (Utilities|String|EnumtoString _output_get)))
  (Utilities|Map|Add (Variables|/Game/Blueprints/Framework/BP_OnlineGameInstance.BP_OnlineGameInstance_C|GetConnectionToClass _asbp_online_game_instance) (PlayerState|GetUniqueID) _output_get))

(fn ConstructionScript)

(fn OnRepIsReady
  (if (Variables|Default|GetIsReady)
    (Development|PrintString (Utilities|String|Append (PlayerState|GetPlayerName) " is now ready") true true "(R=0.000000,G=0.660000,B=1.000000,A=1.000000)" 5.0)
    (else
      (Development|PrintString (Utilities|String|Append (PlayerState|GetPlayerName) " NOT ready") true true "(R=0.000000,G=0.660000,B=1.000000,A=1.000000)" 5.0)))
  (Networking|SwitchHasAuthority
    (:Authority
      (bind _asbp_lobby_game_state (Utilities|Casting|CastToBP_LobbyGameState (Game|GetGameState)))
      (Default|ServerCheckStartCountdown _asbp_lobby_game_state))))

(fn OnRepPickedClass
  (Development|PrintString (Utilities|String|Append (PlayerState|GetPlayerName) " picked class " (Utilities|String|EnumtoString (Variables|Default|GetPickedClass))) true true "(R=0.000000,G=0.660000,B=1.000000,A=1.000000)" 5.0)
  (Networking|SwitchHasAuthority
    (:Authority
      (bind _asbp_lobby_player_controller (Utilities|Casting|CastToBP_LobbyPlayerController (Game|GetPlayerController)))
      (Default|ChangeClassActor _asbp_lobby_player_controller (Variables|Default|GetPickedClass)))))