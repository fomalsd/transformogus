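; Lobby PlayerState that holds each player's picked class and ready state.
; Server events set both RepNotify variables, with readiness only ever set to true here.
; Their OnRep functions print the change with the player's name.
; The ready OnRep also has the authority side ask BP_LobbyGameState to check whether to start the countdown, relying on Blueprint RepNotifies firing on the server.
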(event Custom|Server_SetReady
  (Variables|Default|SetIsReady true))

(event Custom|Server_SetClass
  (params (PlayerClass :type E_PlayerClass%20Enum :default "NewEnumerator0"))
  (Variables|Default|SetPickedClass PlayerClass))

(fn ConstructionScript)

(fn OnRepIsReady
  (if (Variables|Default|GetIsReady)
    (Development|PrintString (Utilities|String|Append (PlayerState|GetPlayerName) " is now ready") true true "(R=0.000000,G=0.660000,B=1.000000,A=1.000000)" 5.0)
    (else
      (Development|PrintString (Utilities|String|Append (PlayerState|GetPlayerName) " NOT ready") true true "(R=0.000000,G=0.660000,B=1.000000,A=1.000000)" 5.0)))
  (Networking|SwitchHasAuthority
    (:Authority
      (bind _asbp_lobby_game_state (Utilities|Casting|CastToBP_LobbyGameState (Game|GetGameState)))
      (Default|ServerCheckStartCountdown _asbp_lobby_game_state))))

(fn OnRepPickedClass
  (Development|PrintString (Utilities|String|Append (PlayerState|GetPlayerName) " picked class " (Utilities|String|EnumtoString (Variables|Default|GetPickedClass))) true true "(R=0.000000,G=0.660000,B=1.000000,A=1.000000)" 5.0))