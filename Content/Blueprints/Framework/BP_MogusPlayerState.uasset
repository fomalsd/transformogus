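; BP_MogusPlayerState is the player state that holds each player's class and ability.
; Server-named events set both values, and their OnRep functions print the player name with the new value for debugging.
; On authority, the ability OnRep also calls ServerCheckPickTraitor on BP_MogusGameState, relying on Blueprint RepNotify also firing on the server, so each ability assignment triggers the traitor-pick check.
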(event Custom|Server_SetAbility
  (params (Player%20Ability :type E_PlayerAbility%20Enum :default "NewEnumerator0"))
  (Variables|Default|SetPlayerAbility Player%20Ability))

(event Custom|Server_SetClass
  (params (PlayerClass :type E_PlayerClass%20Enum :default "NewEnumerator0"))
  (Variables|Default|SetPlayerClass PlayerClass))

(event EventBeginPlay)

(event EventTick
  (params (DeltaSeconds :type Float%20%28single-precision%29)))

(fn ConstructionScript)

(fn OnRepPlayerClass
  (Development|PrintString (Utilities|String|Append (PlayerState|GetPlayerName) " replicated class " (Utilities|String|EnumtoString (Variables|Default|GetPlayerClass)))))

(fn OnRepPlayerAbility
  (Development|PrintString (Utilities|String|Append (PlayerState|GetPlayerName) " got ability " (Utilities|String|EnumtoString (Variables|Default|GetPlayerAbility))))
  (Networking|SwitchHasAuthority
    (:Authority
      (bind _asbp_mogus_game_state (Utilities|Casting|CastToBP_MogusGameState (Game|GetGameState)))
      (Default|ServerCheckPickTraitor _asbp_mogus_game_state))))