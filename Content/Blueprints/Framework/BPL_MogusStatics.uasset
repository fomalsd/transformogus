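; BPL_MogusStatics is a Blueprint function library providing ConeTrace, a helper that returns the actors inside a cone.
; It gathers candidates with a sphere overlap at the origin, using the cone length as radius and the given object types and ignore list.
; It keeps actors whose location lies within half the cone angle of the direction, via dot product and arccosine.
; Each call also draws a one-second debug cone.
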(fn ConeTrace
  (params (WorldContextObject :type Object%20Object%20Reference) (Origin :type Vector) (Direction :type Vector) (Length :type Float%20%28single-precision%29) (Angle :type Float%20%28single-precision%29) (LineColor :type Linear%20Color%20Structure) (ObjectTypes :type Array%20of%20EObjectTypeQuery%20Enums :default "ObjectTypeQuery1") (ActorsToIgnore :type Array%20of%20Actor%20Object%20References))
  (LocalVariables|SetHalfAngle (/ Angle 2.0)) ; either I am dumb or the entire world is fucking dumb
  (Class|KismetSystemLibrary|DrawDebugConeinDegrees WorldContextObject Origin Direction Length (LocalVariables|GetHalfAngle) (LocalVariables|GetHalfAngle) 12 LineColor 1.0 0.0)
  (bind _outactors (Collision|SphereOverlapActors WorldContextObject Origin Length ObjectTypes 0 ActorsToIgnore))
  (for _array_element _outactors
    (if (<= (Class|KismetMathLibrary|DegAcos (Math|Vector|DotProduct Direction (Math|Vector|GetUnitDirection(Vector) Origin (Transformation|GetActorLocation _array_element)))) (LocalVariables|GetHalfAngle))
      (Utilities|Array|Add (LocalVariables|GetHitActors) _array_element)))
  (return (LocalVariables|GetHitActors)))