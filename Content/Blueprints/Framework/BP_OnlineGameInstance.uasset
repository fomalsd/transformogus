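; Online game instance that manages multiplayer rooms, persistent menu music and lookup of the picked class's character, falling back to BP_HealChar.
; HostSession creates an Advanced Sessions room tagged with API version and host-based name, then opens L_Lobby as a listen server.
; StartSession updates that session to lock the room, JoinSession joins a search result, and LeaveSession destroys the session, optionally loading the main menu.
; Version-filtered room search and older hosting logic are disabled.
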(event Custom|HostSession
  (params (UseLAN :type Boolean))
  (Variables|Default|SetSessionUseLAN UseLAN)
  (Variables|Default|SetTemp_RoomName (Utilities|String|ToString(Text) (Utilities|Text|FormatText "Room by {playerName}" (PlayerState|GetPlayerName (Variables|/Script/Engine.Controller|GetPlayerState (Game|GetPlayerController 0))))))
  (Development|PrintString "Creating session...")
  (Variables|Default|SetSessionExtraSettings (Utilities|Array|MakeArray (Class|AdvancedSessionsLibrary|MakeLiteralSessionPropertyInt "transformogusApi" (Variables|Default|GetApiLevel)) (Class|AdvancedSessionsLibrary|MakeLiteralSessionPropertyString "GameSession" (Variables|Default|GetTemp_RoomName))))
  (|AdvancedSession (Utilities|Array|MakeArray (Class|AdvancedSessionsLibrary|MakeLiteralSessionPropertyInt "transformogusApi" (Variables|Default|GetApiLevel)) (Class|AdvancedSessionsLibrary|MakeLiteralSessionPropertyString "GameSession" (Variables|Default|GetTemp_RoomName))) (Game|GetPlayerController 0) (Variables|Default|GetMaxPlayers) 0 (Variables|Default|GetSessionUseLAN) true false true true true false false false true true true
    (:OnSuccess
      (Development|PrintString (Utilities|String|Append "Create session OK! Name:" (Variables|Default|GetTemp_RoomName)))
      (Game|OpenLevel(byObjectReference) "/Game/Maps/L_Lobby.L_Lobby" true "listen"))
    (:OnFailure
      (Development|PrintString "Create session failure!"))))

(event Custom|JoinSession
  (params (Session :type Blueprint%20Session%20Result%20Structure%20%28by%20ref%29))
  (|JoinSession (Game|GetPlayerController 0) Session
    (:OnFailure
      (Development|PrintString "Join session failure!"))))

(event Custom|OnHostResult
  (params (Successful :type Boolean))
  ;[0.06354 0.06354 0.06354] old HostSession
  (if Successful
    (Game|OpenLevel(byObjectReference) "/Game/Maps/L_Lobby.L_Lobby" true "listen")
    (else
      (Development|PrintString "Create session failure!"))))

(event Custom|RefreshSessions
  (bind _results (|FindSessionsAdvanced (Game|GetPlayerController 0) 100 false "AllServers" (Utilities|Array|MakeArray (Class|AdvancedSessionsLibrary|MakeLiteralSessionSearchProperty (Class|AdvancedSessionsLibrary|MakeLiteralSessionPropertyInt "transformogusApi" (Variables|Default|GetApiLevel)) "Equals")) false false false true)
    (:OnSuccess
      (Default|CallOnRoomRefreshResult _results))))

(event Custom|LeaveSession
  (params (LoadMainMenu :type Boolean))
  (|DestroySession (Game|GetPlayerController 0)
    (:then
      (Development|PrintString "Destroying session")
      (if LoadMainMenu
        (Game|OpenLevel(byObjectReference) "/Game/Maps/L_MainMenu.L_MainMenu")))))

(event Custom|PlayMenuMusic
  (bind _returnvalue (Audio|SpawnSound2D "/Game/Sounds/Music/punch-deck-bhangra-bass_Cue.punch-deck-bhangra-bass_Cue" 1.0 1.0 0.0 0 true))
  (bind _output_get (Variables|Default|SetMusic _returnvalue))
  (Audio|Components|Audio|Play _output_get 0.0))

(event Custom|StopMenuMusic
  (bind _music (Variables|Default|GetMusic)
    (:then
      (Audio|Components|Audio|Stop _music))
    (:else)))

(event Custom|StartSession
  (|UpdateSession (Variables|Default|GetSessionExtraSettings) (Variables|Default|GetMaxPlayers) 0 (Variables|Default|GetSessionUseLAN) true false true false
    (:OnSuccess
      (Development|PrintString "Locked the doors, this is a private room now baby"))
    (:OnFailure
      (Development|PrintString "Update session failure!"))))

(fn GetCharacterClass
  (bind _pickedclass (Variables|Default|GetPickedClass))
  (bind _classtocharacter (Variables|Default|GetClassToCharacter))
  (bind (_value _returnvalue) (Utilities|Map|Find _classtocharacter _pickedclass))
  (if _returnvalue
    (return _value)
    (else
      (Development|PrintString (Utilities|String|Append "PickedClass " (Utilities|String|EnumtoString _pickedclass) " character: " (Utilities|GetClassDisplayName _value)))
      (return "/Game/Blueprints/Characters/PlayerCharacters/Healer/BP_HealChar.BP_HealChar_C"))))