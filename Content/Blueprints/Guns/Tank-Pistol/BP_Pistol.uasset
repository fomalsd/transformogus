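; BP_Pistol is a hitscan pistol with limited ammo, reusing shotgun sounds and damage variable.
; ShotPistol spends a round, then line-traces on Visibility from the ShootPoint socket along camera forward, with debug drawing, and damages the hit actor.
; Reload plays a sound and refills ammo after a delay.
; Reload sets IsRealoding false at both ends, so it never blocks firing, and emptying the magazine triggers nothing.
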(event Custom|ShotPistol
  (bind _gun (Variables|Default|GetGun))
  (bind _returnvalue (Transformation|GetSocketLocation _gun "ShootPoint"))
  (if (not (Variables|Default|GetIsRealoding))
    (if (not (<= (Variables|Default|GetAmmo) 0.0))
      (Variables|Default|SetAmmo (- (Variables|Default|GetAmmo) 1.0))
      (Audio|PlaySoundatLocation "/Game/Sounds/Guns/Shotgun/SC_ShotgunShot.SC_ShotgunShot" (Transformation|GetWorldLocation (Variables|Default|GetGun)) "0, 0, 0" 1.0 1.0 0.0 0 0 0 0)
      (bind _outhit (Collision|LineTraceByChannel _returnvalue (+ _returnvalue (* (Math|Vector|GetForwardVector (Variables|/Script/Engine.PlayerCameraManager|GetTransformComponent (Game|GetPlayerCameraManager 0))) (Variables|Default|GetPistolRange))) "TraceTypeQuery1" false 0 "ForDuration"))
      (Game|Damage|ApplyDamage (.HitActor (Collision|BreakHitResult _outhit)) (Variables|Default|GetShotGunDamage) 0 0)
      (if (<= (Variables|Default|GetAmmo) 0.0)
        _))))

(event Custom|Reload
  (Variables|Default|SetIsRealoding false)
  (Audio|SpawnSoundatLocation "/Game/Sounds/Guns/Shotgun/SC_ShotgunReload.SC_ShotgunReload" (Transformation|GetWorldLocation (Variables|Default|GetGun)) "0, 0, 0" 1.0 1.0 0.0 0 0)
  (Utilities|FlowControl|Delay (Variables|Default|GetReloadTimer))
  (Variables|Default|SetAmmo (Variables|Default|GetFullAmmo))
  (Variables|Default|SetIsRealoding false))

(event EventBeginPlay
  (Variables|Default|SetAmmo (Variables|Default|GetFullAmmo)))

(fn ConstructionScript
  (|CallParentFunction))