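; Engineer shotgun weapon that fires hitscan pellet bursts and manages its own ammo and timed reload.
; ShotgunShot spends ammo and fires randomly spread line traces from the ShootPoint socket along the camera forward, damaging hit actors and drawing debug traces.
; The gun's material swaps when ammo runs out; firing while empty calls Reload, which restores the emissive material and refills ammo after a delay.
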(event Custom|ShotgunShot
  (bind _shotgunspread (Variables|Default|GetShotGunSpread))
  (bind _shotgunspread_2 (Variables|Default|GetShotGunSpread))
  (bind _gun (Variables|Default|GetGun))
  (bind _shotgunspread_3 (Variables|Default|GetShotGunSpread))
  (bind _returnvalue (Transformation|GetSocketLocation _gun "ShootPoint"))
  (if (not (Variables|Default|GetIsReloading))
    (if (<= (Variables|Default|GetGAmmo) 0.0)
      (CallFunction|Reload)
      (else
        (Variables|Default|SetGAmmo (- (Variables|Default|GetGAmmo) 1.0))
        (Audio|PlaySoundatLocation "/Game/Sounds/Guns/Shotgun/SC_ShotgunShot.SC_ShotgunShot" (Transformation|GetWorldLocation (Variables|Default|GetGun)) "0, 0, 0" 1.0 1.0 0.0 0 0 0 0)
        (for _index (range 0 11)
          (bind _outhit (Collision|LineTraceByChannel _returnvalue (+ _returnvalue (* (Math|Vector|GetForwardVector (Variables|/Script/Engine.PlayerCameraManager|GetTransformComponent (Game|GetPlayerCameraManager 0))) (Variables|Default|GetShotGunRange)) (Math|Vector|MakeVector (Math|Random|RandomFloatinRange (* _shotgunspread -1.0) _shotgunspread) (Math|Random|RandomFloatinRange (* _shotgunspread_2 -1.0) _shotgunspread_2) (Math|Random|RandomFloatinRange (* _shotgunspread_3 -1.0) _shotgunspread_3))) "TraceTypeQuery1" false 0 "ForDuration"))
          (Game|Damage|ApplyDamage (.HitActor (Collision|BreakHitResult _outhit)) (Variables|Default|GetShotGunDamage) 0 0)
          (if (<= (Variables|Default|GetGAmmo) 0.0)
            (Rendering|Material|SetMaterial (Variables|Default|GetGun) 1 "/Engine/VREditor/UI/DiscMaterial.DiscMaterial")))))))

(event Custom|Reload
  (Variables|Default|SetIsReloading true)
  (Rendering|Material|SetMaterial (Variables|Default|GetGun) 1 "/Game/Guns/Tank/Military/Emission_001.Emission_001")
  (Audio|SpawnSoundatLocation "/Game/Sounds/Guns/Shotgun/SC_ShotgunReload.SC_ShotgunReload" (Transformation|GetWorldLocation (Variables|Default|GetGun)) "0, 0, 0" 1.0 1.0 0.0 0 0)
  (Utilities|FlowControl|Delay (Variables|Default|GetReloadTimer))
  (Variables|Default|SetGAmmo (Variables|Default|GetFullAmmo))
  (Variables|Default|SetIsReloading false))

(event EventBeginPlay
  (Variables|Default|SetGAmmo (Variables|Default|GetFullAmmo)))

(fn ConstructionScript
  (|CallParentFunction))

(fn OnRepAmmo)