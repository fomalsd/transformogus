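; BP_EngineerChar is the Engineer player character, armed with a shotgun and able to place turrets.
; On BeginPlay it spawns a BP_ShotGun and attaches it to the mesh's right-hand gun socket.
; Left mouse fires the shotgun and plays a fire montage.
; Right mouse spawns a BP_TurretEngineer at a fixed world-X offset from the mesh, matching its rotation, and prints the turret's location.
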(event EventBeginPlay
  (bind _mesh (Variables|Character|GetMesh))
  (|CallParentFunction)
  (bind _returnvalue (Game|SpawnActorfromClass "/Game/Blueprints/Guns/Engineer-ShotGun/BP_ShotGun.BP_ShotGun_C" (Math|Transform|MakeTransform (Transformation|GetSocketLocation _mesh "RHGunSocket")) "Undefined" "MultiplyWithRoot" 0 0))
  (bind _output_get (Variables|Default|SetShotGun _returnvalue))
  (Transformation|AttachComponentToComponent _output_get _mesh "RHGunSocket" "SnapToTarget" "KeepRelative" "KeepRelative" true))

(event Collision|EventActorBeginOverlap
  (params (OtherActor :type Actor%20Object%20Reference))
  (|CallParentFunction OtherActor) ; This node is disabled and will not be called.\nDrag off pins to build functionality.
)

(event EventTick
  (params (DeltaSeconds :type Float%20%28single-precision%29))
  (|CallParentFunction DeltaSeconds) ; This node is disabled and will not be called.\nDrag off pins to build functionality.
)

(event Input|MouseEvents|LeftMouseButton
  (params (Key :type Key%20Structure :default "None"))
  (:Pressed
    (Default|ShotgunShot (Variables|Default|GetShotGun))
    (Animation|Montage|PlayMontage (Variables|Character|GetMesh) (Variables|Animations|GetFireMontage))))

(event Input|MouseEvents|RightMouseButton
  (params (Key :type Key%20Structure :default "None"))
  (bind _mesh (Variables|Character|GetMesh))
  (bind _returnvalue (Transformation|GetWorldLocation _mesh))
  (:Pressed
    (bind _returnvalue_2 (Game|SpawnActorfromClass "/Game/Blueprints/Characters/PlayerCharacters/Engineer/BP_TurretEngineer.BP_TurretEngineer_C" (Math|Transform|MakeTransform (Math|Vector|MakeVector (+ (.x _returnvalue) 1e+02) (.y _returnvalue) (.z _returnvalue)) (Transformation|GetWorldRotation _mesh) "1.000000,1.000000,1.000000") "AdjustIfPossibleButAlwaysSpawn" "MultiplyWithRoot" 0 0))
    (Development|PrintString (Utilities|String|ToString(Vector) (Transformation|GetActorLocation _returnvalue_2)))))

(fn ConstructionScript
  (|CallParentFunction))