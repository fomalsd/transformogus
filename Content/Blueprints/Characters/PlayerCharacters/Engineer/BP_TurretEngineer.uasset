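; Engineer turret actor that starts firing on BeginPlay through repeated line traces, with no hit handling or damage yet.
; StartShootTurret runs a debug-drawn Visibility trace from each Turret socket to the forward vector scaled by TurretRange, without adding the socket location.
; Inside that loop it sets a timer on itself using TurretLiveTimer, so firing repeats at that interval.
; DestroyActor is unconnected, so the turret never destroys itself here.
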(event Custom|StartShootTurret
  (bind _turret (Variables|Default|GetTurret))
  (for _array_element (Transformation|GetAllSocketNames (Variables|Default|GetTurret))
    (Collision|LineTraceByChannel (Transformation|GetSocketLocation _turret _array_element) (* (Math|Vector|GetForwardVector _turret) (Variables|Default|GetTurretRange)) "TraceTypeQuery1" false 0 "ForDuration")
    (Utilities|Time|SetTimerbyEvent (delegate Custom|StartShootTurret) (Variables|Default|GetTurretLiveTimer))))

(event EventBeginPlay
  (CallFunction|StartShootTurret))

(event Collision|EventActorBeginOverlap
  (params (OtherActor :type Actor%20Object%20Reference)))

(event EventTick
  (params (DeltaSeconds :type Float%20%28single-precision%29)))

(fn ConstructionScript)