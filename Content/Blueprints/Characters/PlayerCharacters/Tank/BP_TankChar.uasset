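; BP_TankChar is the Tank player character, adding a pistol and health handling on top of its parent class.
; BeginPlay resets health to max, then spawns BP_Pistol and attaches it to the mesh's "PistolSocked" socket.
; Left mouse and R forward to the pistol's shoot and reload.
; Damage lowers health, and at zero or below it destroys the mesh and calls Death, a path the 1 key also triggers directly.
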(event EventBeginPlay
  (bind _mesh (Variables|Character|GetMesh))
  (Variables|Default|SetTankCurrentHealth (Variables|Default|GetTankMaxHealth))
  (|CallParentFunction)
  (bind _returnvalue (Game|SpawnActorfromClass "/Game/Blueprints/Guns/Tank-Pistol/BP_Pistol.BP_Pistol_C" (Math|Transform|MakeTransform (Transformation|GetSocketLocation _mesh "PistolSocked")) "Undefined" "MultiplyWithRoot" 0 0))
  (bind _output_get (Variables|Default|SetPistol _returnvalue))
  (Transformation|AttachComponentToComponent _output_get _mesh "PistolSocked" "SnapToTarget" "KeepRelative" "KeepRelative" true))

(event Collision|EventActorBeginOverlap
  (params (OtherActor :type Actor%20Object%20Reference))
  (|CallParentFunction OtherActor) ; This node is disabled and will not be called.\nDrag off pins to build functionality.
)

(event EventTick
  (params (DeltaSeconds :type Float%20%28single-precision%29))
  (|CallParentFunction DeltaSeconds) ; This node is disabled and will not be called.\nDrag off pins to build functionality.
)

(event Game|Damage|EventAnyDamage
  (params (Damage :type Float%20%28single-precision%29) (DamageType :type Damage%20Type%20Object%20Reference) (InstigatedBy :type Controller%20Object%20Reference) (DamageCauser :type Actor%20Object%20Reference))
  (bind _output_get (Variables|Default|SetTankCurrentHealth (- (Variables|Default|GetTankCurrentHealth) Damage)))
  (if (<= _output_get 0.0)
    (Components|DestroyComponent (Variables|Character|GetMesh))
    (CallFunction|Death)))

(event Input|KeyboardEvents|R
  (params (Key :type Key%20Structure :default "None"))
  (:Pressed
    (Default|Reload (Variables|Default|GetPistol))))

(event Input|MouseEvents|LeftMouseButton
  (params (Key :type Key%20Structure :default "None"))
  (:Pressed
    (Default|ShotPistol (Variables|Default|GetPistol))))

(event Input|KeyboardEvents|1
  (params (Key :type Key%20Structure :default "None"))
  (:Pressed
    (Components|DestroyComponent (Variables|Character|GetMesh))
    (CallFunction|Death)))

(fn ConstructionScript
  (|CallParentFunction))