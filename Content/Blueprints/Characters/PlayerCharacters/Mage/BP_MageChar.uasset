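; BP_MageChar is the Mage player character, which fights with a glove weapon.
; On BeginPlay it spawns a BP_Glove actor at the mesh's GloveSocket, stores it and attaches it to that socket.
; Left mouse fires the glove and R reloads it, both by calling straight into the glove, so the character holds no shot or reload logic itself.
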(event EventBeginPlay
  (bind _mesh (Variables|Character|GetMesh))
  (|CallParentFunction)
  (bind _returnvalue (Game|SpawnActorfromClass "/Game/Blueprints/Guns/Mage-Glove/BP_Glove.BP_Glove_C" (Math|Transform|MakeTransform (Transformation|GetSocketLocation _mesh "GloveSocket")) "Undefined" "MultiplyWithRoot" 0 0))
  (bind _output_get (Variables|Default|SetGlove _returnvalue))
  (Transformation|AttachComponentToComponent _output_get _mesh "GloveSocket" "SnapToTarget" "KeepRelative" "KeepRelative" true))

(event Collision|EventActorBeginOverlap
  (params (OtherActor :type Actor%20Object%20Reference))
  (|CallParentFunction OtherActor) ; This node is disabled and will not be called.\nDrag off pins to build functionality.
)

(event EventTick
  (params (DeltaSeconds :type Float%20%28single-precision%29))
  (|CallParentFunction DeltaSeconds) ; This node is disabled and will not be called.\nDrag off pins to build functionality.
)

(event Input|MouseEvents|LeftMouseButton
  (params (Key :type Key%20Structure))
  (:Pressed
    (Default|GloveShot (Variables|Default|GetGlove))))

(event Input|KeyboardEvents|R
  (params (Key :type Key%20Structure))
  (:Pressed
    (Default|Reload (Variables|Default|GetGlove))))

(fn ConstructionScript
  (|CallParentFunction))