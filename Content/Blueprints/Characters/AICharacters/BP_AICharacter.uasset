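; BP_AICharacter is an AI character Blueprint that finds the nearest player character when play begins.
; FindNearestPlayer loops over all BP_Character actors, using a shrinking distance threshold to store the closest one within 2000 units in ClosestPlayer.
; The search runs only on BeginPlay, and nothing in these graphs acts on the stored result.
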(event Custom|FindNearestPlayer
  (Variables|Default|SetClosesPlayer 2e+03)
  (bind _outactors (Actor|GetAllActorsOfClass "/Game/Blueprints/Characters/BP_Character.BP_Character_C"))
  (for _array_element _outactors
    (if (< (Transformation|GetDistanceTo _array_element self) (Variables|Default|GetClosesPlayer))
      (Variables|Default|SetClosesPlayer (Transformation|GetDistanceTo _array_element self))
      (Variables|Default|SetClosestPlayer _array_element))))

(event EventBeginPlay
  (CallFunction|FindNearestPlayer))

(event Collision|EventActorBeginOverlap
  (params (OtherActor :type Actor%20Object%20Reference)))

(event EventTick
  (params (DeltaSeconds :type Float%20%28single-precision%29)))

(fn ConstructionScript)