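; Enemy creep character that picks the nearest target and reacts to elemental damage types.
; AnyDamage branches by type: fire burns over time, air launches, water slows, earth roots, bullets only damage, and love temporarily retargets to spawn points without pawn collision.
; ReduceHealth triggers death at zero, reporting the kill to BP_MogusGameState and ragdolling before destruction.
; Water's slow is never reset after its delay, unlike earth's.
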(event Custom|FindNearestPlayer
  ;[1 1 1] FindNearestPlayer
  (bind _output_get (Variables|Pathfinding|SetClosestTargetRange (Variables|Pathfinding|GetTargetRange)))
  (bind _outactors (Actor|GetAllActorsOfClass (Variables|Pathfinding|GetFollowTarget)))
  (for _array_element _outactors
    (if (< (Transformation|GetDistanceTo _array_element self) (Variables|Pathfinding|GetClosestTargetRange))
      (Variables|Pathfinding|SetClosestTargetRange (Transformation|GetDistanceTo _array_element self))
      (bind _output_get_2 (Variables|Pathfinding|SetClosestTarget _array_element))
      (Development|PrintString (Utilities|String|Append "targeting " (Utilities|GetDisplayName _output_get_2))))))

(event Custom|Multicast_PlaySound
  (params (SoundToPlay :type Sound%20Base%20Object%20Reference))
  ;[1 1 1] Damage
  (bind _returnvalue (Audio|SpawnSoundatLocation SoundToPlay (Transformation|GetActorLocation) "0, 0, 0" 1.0 1.0 0.0 0 0))
  (Audio|Components|Audio|Play _returnvalue 0.0))

(event Custom|Ignite
  (params (FireStaySeconds :type Float%20%28double-precision%29))
  (Utilities|FlowControl|Sequence
    (:then_0
      (Variables|Default|SetIsBurning true)
      (Utilities|FlowControl|Delay FireStaySeconds)
      (Variables|Default|SetIsBurning false))
    (:then_1
      (if (Variables|Default|GetIsBurning) :!label _label
        (Networking|SwitchHasAuthority
          (:Authority
            (CallFunction|ReduceHealth 5.0) ; todo use table
          )
          (:Remote
            _))
        (CallFunction|PlayBurnFX)
        (Utilities|FlowControl|Delay 1.0)
        (goto _label)))))

(event Custom|Multicast_SetCollision
  (params (CollisionState :type ECollisionResponse%20Enum :default "ECR_Ignore"))
  ;[1 1 1] Damage
  (Collision|SetCollisionResponsetoChannel (Variables|Collision|GetCapsuleComponent) "ECC_Pawn" CollisionState))

(event Custom|CreepDeath
  ;[1 1 1] Death
  (bind _asbp_mogus_game_state (Utilities|Casting|CastToBP_MogusGameState (Game|GetGameState)))
  (Default|ServerReportCreepKill _asbp_mogus_game_state)
  (Collision|SetCollisionEnabled (Variables|Collision|GetCapsuleComponent) "NoCollision")
  (Physics|SetSimulatePhysics (Variables|Character|GetMesh) true)
  (Utilities|FlowControl|Delay 3.0)
  (Actor|DestroyActor))

(event EventBeginPlay
  (Variables|Default|SetCurrentHealth (Variables|Default|GetMaxHealth))
  (Variables|Pathfinding|SetTargetRange (Variables|Pathfinding|GetPlayerDetectRange))
  (CallFunction|FindNearestPlayer)
  (Variables|Default|SetOriginalMaxSpeed (Variables|/Script/Engine.CharacterMovementComponent|GetMaxWalkSpeed (Variables|Character|GetCharacterMovement))))

(event Game|Damage|EventAnyDamage
  (params (Damage :type Float%20%28single-precision%29) (DamageType :type Damage%20Type%20Object%20Reference) (InstigatedBy :type Controller%20Object%20Reference) (DamageCauser :type Actor%20Object%20Reference))
  ;[1 1 1] Damage
  (Utilities|FlowControl|Sequence
    (:then_0
      (bind _asfire_damage (Utilities|Casting|CastToFireDamage DamageType))
      (CallFunction|Ignite (Default|GetEffectDuration _asfire_damage))
      (CallFunction|ReduceHealth Damage))
    (:then_1
      (Utilities|Casting|CastToAirDamage DamageType)
      (CallFunction|FlyUp DamageCauser)
      (CallFunction|ReduceHealth Damage))
    (:then_2
      (bind _aswater_damage (Utilities|Casting|CastToWaterDamage DamageType))
      (CallFunction|SetSpeed 0.25)
      (CallFunction|PlayWaterFX)
      (CallFunction|ReduceHealth Damage)
      (Utilities|FlowControl|Delay (Default|GetEffectDuration _aswater_damage)))
    (:then_3
      (bind _asearth_damage (Utilities|Casting|CastToEarthDamage DamageType))
      (CallFunction|SetSpeed 0.0)
      (CallFunction|PlayEarthFreezeFX)
      (CallFunction|ReduceHealth Damage)
      (Utilities|FlowControl|Delay (Default|GetEffectDuration _asearth_damage))
      (CallFunction|SetSpeed 1.0))
    (:then_4
      (bind _aslove_damage (Utilities|Casting|CastToLoveDamage DamageType))
      (CallFunction|PlayLoveSFX)
      (Variables|Default|SetTemp_CollisionState (Collision|GetCollisionResponsetoChannel (Variables|Collision|GetCapsuleComponent) "ECC_Pawn"))
      (CallFunction|MulticastSetCollision "ECR_Ignore")
      (Utilities|Array|Add (Variables|Default|GetIgnoredActors) InstigatedBy)
      (Variables|Pathfinding|SetTargetRange (Variables|Pathfinding|GetSpawnDetectRange))
      (Variables|Pathfinding|SetFollowTarget "/Game/Blueprints/EnemySpawner/BP_CreepSpawnPoint.BP_CreepSpawnPoint_C")
      (Utilities|FlowControl|Delay (Default|GetEffectDuration _aslove_damage))
      (Variables|Pathfinding|SetFollowTarget (Variables|Pathfinding|GetDefaultFollowTarget))
      (Variables|Pathfinding|SetTargetRange (Variables|Pathfinding|GetPlayerDetectRange))
      (CallFunction|MulticastSetCollision (Variables|Default|GetTemp_CollisionState)))
    (:then_5
      (Utilities|Casting|CastToBulletDamage DamageType)
      (CallFunction|ReduceHealth Damage))))

(fn ConstructionScript)

(fn ReduceHealth
  (params (Damage :type Float%20%28double-precision%29))
  (Rendering|Decal|SpawnDecalatLocation "/Game/Guns/Healer/Wizzard/Textures/Emission/Syringe_Wizzard_Painter_Emisiion_OcclusionRoughnessMetallic_Mat.Syringe_Wizzard_Painter_Emisiion_OcclusionRoughnessMetallic_Mat" "30.000000,30.000000,30.000000" (Transformation|GetActorLocation) "-90.000000,0.000000,0.000000" 1.0)
  (bind _output_get (Variables|Default|SetCurrentHealth (- (Variables|Default|GetCurrentHealth) Damage)))
  (if (<= _output_get 0.0)
    (CallFunction|CreepDeath)))

(fn SetSpeed
  (params (SpeedMult :type Float%20%28double-precision%29))
  (bind _charactermovement (Variables|Character|GetCharacterMovement))
  (bind _originalmaxspeed (Variables|Default|GetOriginalMaxSpeed))
  (bind _returnvalue (* _originalmaxspeed SpeedMult))
  (Variables|/Script/Engine.CharacterMovementComponent|SetMaxCustomMovementSpeed _charactermovement _returnvalue)
  (Variables|/Script/Engine.CharacterMovementComponent|SetMaxWalkSpeed _charactermovement _returnvalue))

(fn PlayLoveSFX
  (CallFunction|MulticastPlaySound "/Game/Sounds/Abilities/love_Cue.love_Cue"))

(fn FlyUp
  (params (DamageCauser :type Actor%20Object%20Reference))
  (bind _returnvalue (Transformation|GetActorLocation))
  (bind _returnvalue_2 (Transformation|GetActorLocation DamageCauser))
  (bind _returnvalue_3 (Math|Vector|GetUnitDirection(Vector) _returnvalue_2 _returnvalue))
  (bind _returnvalue_4 (+ _returnvalue_3 "0.000000,0.000000,5.000000"))
  (bind _returnvalue_5 (* _returnvalue_4 "200.000000,200.000000,200.000000"))
  (CallFunction|MulticastPlaySound "/Game/Sounds/Abilities/pitfall_Cue.pitfall_Cue")
  (Variables|/Script/Engine.MovementComponent|SetVelocity (Variables|Character|GetCharacterMovement) _returnvalue_5)
  (Character|LaunchCharacter _returnvalue_5 false true)
  (Physics|AddImpulse (Variables|Character|GetCharacterMovement) _returnvalue_5 false))

(fn PlayEarthFreezeFX
  (CallFunction|MulticastPlaySound "/Game/Sounds/Abilities/earth_Cue.earth_Cue"))

(fn PlayWaterFX
  (CallFunction|MulticastPlaySound "/Game/Sounds/Abilities/water_Cue.water_Cue"))

(fn PlayBurnFX
  (CallFunction|MulticastPlaySound "/Game/Sounds/Abilities/fire_Cue.fire_Cue"))