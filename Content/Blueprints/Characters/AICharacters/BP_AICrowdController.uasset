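; AI controller that makes a BP_Enemy pawn chase the nearest player.
; On BeginPlay it runs FindPlayer at once and again on a one-second looping timer.
; Each pass asks the enemy to find its nearest player, then issues AI MoveTo toward that ClosestTarget.
; The Niagara spawn and pawn destruction on reaching the target are disabled, and Tick is unused.
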(event Custom|Find%20player
  (bind _returnvalue (Pawn|GetControlledPawn))
  (bind _asbp_enemy (Utilities|Casting|CastToBP_Enemy _returnvalue))
  (Default|FindNearestPlayer _asbp_enemy)
  (AI|AIMoveTo 0 "0, 0, 0" (Variables|/Game/Blueprints/Characters/AICharacters/BP_Enemy.BP_Enemy_C|GetClosestTarget _asbp_enemy) 5.0 false
    (:OnSuccess
      (Niagara|SpawnSystematLocation "/Game/FX/NewNiagaraSystem.NewNiagaraSystem" (Transformation|GetActorLocation _returnvalue))
      (Actor|DestroyActor _returnvalue))))

(event EventBeginPlay
  (Utilities|Time|SetTimerbyEvent (delegate Custom|Find%20player) 1.0 true)
  (CallFunction|FindPlayer))

(event EventTick
  (params (DeltaSeconds :type Float%20%28single-precision%29)))

(fn ConstructionScript)