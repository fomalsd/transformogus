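; Networked player character for a game with traitors, with replicated health, a client-created HUD and a boss transformation.
; AnyDamage branches on damage type: fire burns over time, air launches, water slows, earth freezes, love disables pawn collision, bullets only damage.
; ReduceHealth feeds Death, which reports traitor kills to the game state, possesses a spectator and destroys the body.
; Water slow is never reset after its delay; TranceformToMagic is empty.
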(event Custom|Death
  (params (Killer :type Controller%20Object%20Reference) (Actor :type Actor%20Object%20Reference))
  (CallFunction|TryReportTraitorKill Killer)
  (bind _hud (Variables|Default|GetHUD)
    (:then
      (Widget|RemovefromParent _hud))
    (:else
      _))
  (bind _returnvalue (Game|SpawnActorfromClass "/Game/Blueprints/Framework/BP_Spectator.BP_Spectator_C" (Transformation|GetWorldTransform (Variables|Default|GetFollowCamera)) "Undefined" "MultiplyWithRoot" 0 0))
  (Pawn|Possess (Game|GetPlayerController 0) _returnvalue)
  (IElementalDamage|PlayDeathSFX)
  (Utilities|FlowControl|Delay 2.0)
  (Actor|DestroyActor))

(event Custom|Multicast_PlaySound
  (params (SoundToPlay :type Sound%20Base%20Object%20Reference) (SpawnSound :type Boolean))
  (bind _audio (Variables|Default|GetAudio))
  ;[1 1 1] Damage
  (if SpawnSound
    (bind _returnvalue (Audio|SpawnSoundatLocation SoundToPlay (Transformation|GetActorLocation) "0, 0, 0" 1.0 1.0 0.0 0 0))
    (Audio|Components|Audio|Play _returnvalue 0.0)
    (else
      (Audio|Components|Audio|SetSound _audio SoundToPlay)
      (Audio|Components|Audio|Play _audio 0.0))))

(event Custom|Ignite
  (params (FireStaySeconds :type Float%20%28double-precision%29) (Instigator :type Controller%20Object%20Reference))
  ;[1 1 1] Damage
  (Utilities|FlowControl|Sequence
    (:then_0
      (Variables|Default|SetIsBurning true)
      (Utilities|FlowControl|Delay FireStaySeconds)
      (Variables|Default|SetIsBurning false))
    (:then_1
      (if (Variables|Default|GetIsBurning) :!label _label
        (Networking|SwitchHasAuthority
          (:Authority
            (IElementalDamage|ReduceHealth 5.0 Instigator) ; todo use table
          )
          (:Remote
            _))
        (IElementalDamage|PlayBurnFX)
        (Utilities|FlowControl|Delay 1.0)
        (goto _label)))))

(event Custom|Multicast_SetCollision
  (params (NewResponse :type ECollisionResponse%20Enum :default "ECR_Ignore"))
  ;[1 1 1] Damage
  (Collision|SetCollisionResponsetoChannel (Variables|Default|GetCapsuleComponent) "ECC_Pawn" NewResponse))

(event Custom|PlayLocalSound
  (params (NewSound :type Sound%20Base%20Object%20Reference))
  (bind _audio (Variables|Default|GetAudio))
  ;[1 1 1] Damage
  (Audio|Components|Audio|SetSound _audio NewSound)
  (Audio|Components|Audio|Play _audio 0.0))

(event Custom|Client_Create_HUD
  (bind _asplayer_controller (Utilities|Casting|CastToPlayerController (Pawn|GetController)))
  (bind _output_get (Variables|Default|SetAs%20Player%20Controller _asplayer_controller))
  (bind _returnvalue (UserInterface|CreateWidget "/Game/UI/W_HUD.W_HUD_C" _output_get))
  (bind _output_get_2 (Variables|Default|SetHUD _returnvalue))
  (UserInterface|Viewport|AddtoViewport _output_get_2 0)
  (Variables|Default|SetCurrentHealth (Variables|Default|GetMaxHealth)))

(event Custom|TranceformToBoss
  (bind _charactermovement (Variables|Character|GetCharacterMovement))
  (Components|SkeletalMesh|SetSkeletalMeshAsset (Variables|Character|GetMesh) "/Game/Mesh/Characters/Main_Monster/Main_Monster.Main_Monster")
  (Variables|/Script/Engine.CharacterMovementComponent|SetMaxWalkSpeed _charactermovement 9e+02)
  (Variables|/Script/Engine.CharacterMovementComponent|SetJumpZVelocity _charactermovement 1.2e+03))

(event Custom|TranceformToMagic)

(event EventBeginPlay
  (bind _asbp_gun (Utilities|Casting|CastToBP_Gun (Components|GetOwner)))
  (Variables|Default|SetAs%20BP%20Gun _asbp_gun)
  (Variables|Default|SetCurrentHealth (Variables|Default|GetMaxHealth)))

(event EventPossessed
  (params (NewController :type Controller%20Object%20Reference))
  (Utilities|Casting|CastToBP_MogusPlayerController NewController)
  (CallFunction|ClientCreateHUD))

(event Game|Damage|EventAnyDamage
  (params (Damage :type Float%20%28single-precision%29) (DamageType :type Damage%20Type%20Object%20Reference) (InstigatedBy :type Controller%20Object%20Reference) (DamageCauser :type Actor%20Object%20Reference))
  ;[1 1 1] Damage
  (Utilities|FlowControl|Sequence
    (:then_0
      (bind _asfire_damage (Utilities|Casting|CastToFireDamage DamageType))
      (CallFunction|Ignite (Default|GetEffectDuration _asfire_damage) InstigatedBy)
      (IElementalDamage|ReduceHealth Damage InstigatedBy))
    (:then_1
      (Utilities|Casting|CastToAirDamage DamageType)
      (IElementalDamage|FlyUp DamageCauser)
      (IElementalDamage|ReduceHealth Damage InstigatedBy))
    (:then_2
      (bind _aswater_damage (Utilities|Casting|CastToWaterDamage DamageType))
      (IElementalDamage|SetSpeed 0.25)
      (IElementalDamage|PlayWaterFX)
      (IElementalDamage|ReduceHealth Damage InstigatedBy)
      (Utilities|FlowControl|Delay (Default|GetEffectDuration _aswater_damage)))
    (:then_3
      (bind _asearth_damage (Utilities|Casting|CastToEarthDamage DamageType))
      (IElementalDamage|SetSpeed 0.0)
      (IElementalDamage|PlayEarthFreezeFX)
      (IElementalDamage|ReduceHealth Damage InstigatedBy)
      (Utilities|FlowControl|Delay (Default|GetEffectDuration _asearth_damage))
      (IElementalDamage|SetSpeed 1.0))
    (:then_4
      (bind _aslove_damage (Utilities|Casting|CastToLoveDamage DamageType))
      (IElementalDamage|PlayLoveSFX)
      (Variables|IElementalDamage|SetTemp_CollisionState (Collision|GetCollisionResponsetoChannel (Variables|Default|GetCapsuleComponent) "ECC_Pawn"))
      (CallFunction|MulticastSetCollision "ECR_Ignore")
      (Utilities|Array|Add (Variables|IElementalDamage|GetIgnoredActors) InstigatedBy)
      (Utilities|FlowControl|Delay (Default|GetEffectDuration _aslove_damage))
      (CallFunction|MulticastSetCollision (Variables|IElementalDamage|GetTemp_CollisionState)))
    (:then_5
      (Utilities|Casting|CastToBulletDamage DamageType)
      (IElementalDamage|ReduceHealth Damage InstigatedBy))))

(fn ConstructionScript)

(fn ReduceHealth
  (params (Damage :type Float%20%28double-precision%29) (Instigator :type Controller%20Object%20Reference))
  (Rendering|Decal|SpawnDecalatLocation "/Game/Guns/Healer/Wizzard/Textures/Emission/Syringe_Wizzard_Painter_Emisiion_OcclusionRoughnessMetallic_Mat.Syringe_Wizzard_Painter_Emisiion_OcclusionRoughnessMetallic_Mat" "30.000000,30.000000,30.000000" (Transformation|GetActorLocation) "-90.000000,0.000000,0.000000" 1.0)
  (bind _output_get (Variables|Default|SetCurrentHealth (- (Variables|Default|GetCurrentHealth) Damage)))
  (if (<= _output_get 0.0)
    (CallFunction|Death Instigator)))

(fn SetSpeed
  (params (SpeedMult :type Float%20%28double-precision%29))
  (bind _charactermovement (Variables|Character|GetCharacterMovement))
  (bind _originalmaxspeed (Variables|Default|GetOriginalMaxSpeed))
  (bind _returnvalue (* _originalmaxspeed SpeedMult))
  (Variables|/Script/Engine.CharacterMovementComponent|SetMaxCustomMovementSpeed _charactermovement _returnvalue)
  (Variables|/Script/Engine.CharacterMovementComponent|SetMaxWalkSpeed _charactermovement _returnvalue))

(fn PlayLoveSFX
  (CallFunction|MulticastPlaySound "/Game/Sounds/Abilities/love_Cue.love_Cue" false))

(fn FlyUp
  (params (DamageCauser :type Actor%20Object%20Reference))
  (bind _returnvalue (Transformation|GetActorLocation DamageCauser))
  (bind _returnvalue_2 (Transformation|GetActorLocation))
  (bind _audio (Variables|Default|GetAudio))
  (bind _returnvalue_3 (Math|Vector|GetUnitDirection(Vector) _returnvalue _returnvalue_2))
  (bind _returnvalue_4 (+ _returnvalue_3 "0.000000,0.000000,4.000000"))
  (bind _returnvalue_5 (* _returnvalue_4 "200.000000,200.000000,200.000000"))
  (Audio|Components|Audio|SetSound _audio "/Game/Sounds/Abilities/pitfall_Cue.pitfall_Cue")
  (Audio|Components|Audio|Play _audio 0.0)
  (Variables|/Script/Engine.MovementComponent|SetVelocity (Variables|Character|GetCharacterMovement) _returnvalue_5)
  (Character|LaunchCharacter _returnvalue_5 false true)
  (Physics|AddImpulse (Variables|Character|GetCharacterMovement) _returnvalue_5 false))

(fn PlayEarthFreezeFX
  (CallFunction|MulticastPlaySound "/Game/Sounds/Abilities/earth_Cue.earth_Cue" false))

(fn PlayWaterFX
  (CallFunction|MulticastPlaySound "/Game/Sounds/Abilities/water_Cue.water_Cue" false))

(fn PlayBurnFX
  (CallFunction|MulticastPlaySound "/Game/Sounds/Abilities/fire_Cue.fire_Cue" false))

(fn PlayDeathSFX
  (CallFunction|MulticastPlaySound "/Game/Sounds/death_Cue.death_Cue" true))

(fn OnRepCurrentHealth
  (bind _returnvalue (CallFunction|GetHealthPercentage))
  (Default|CallHealthChanged _returnvalue)
  (return))

(fn GetHealthPercentage
  (return (Math|Float|Clamp(Float) (/ (Variables|Default|GetCurrentHealth) (Variables|Default|GetMaxHealth)))))

(fn TryReportTraitorKill
  (params (Object :type Object%20Object%20Reference))
  (bind _asbp_mogus_player_controller (Utilities|Casting|CastToBP_MogusPlayerController Object)
    (:then
      (if (Variables|/Game/Blueprints/Framework/BP_MogusPlayerController.BP_MogusPlayerController_C|GetIsTraitor _asbp_mogus_player_controller)
        (bind _asbp_mogus_game_state (Utilities|Casting|CastToBP_MogusGameState (Game|GetGameState))
          (:then
            (Default|ServerReportTraitorKill _asbp_mogus_game_state))
          (:CastFailed
            _))))
    (:CastFailed
      _))
  (return))