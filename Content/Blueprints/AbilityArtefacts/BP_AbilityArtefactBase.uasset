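; Base pickup artefact that grants its configured Ability to a player who overlaps it.
; On BeginPlay it tints the cube through a dynamic material, using the color from the ability's DT_AbilityStats row.
; The server grants the ability through BP_MogusPlayerState only if the player holds the default enum value, otherwise printing a refusal.
; A successful pickup sets IsConsumed, whose RepNotify destroys the actor.
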(event OnComponentBeginOverlap(OverlapTrigger)
  (params (OverlappedComponent :type Primitive%20Component%20Object%20Reference) (OtherActor :type Actor%20Object%20Reference) (OtherComp :type Primitive%20Component%20Object%20Reference) (OtherBodyIndex :type Integer) (bFromSweep :type Boolean) (SweepResult :type Hit%20Result%20Structure%20%28by%20ref%29))
  (Development|PrintString (Utilities|String|Append "overlap with " (Utilities|GetDisplayName OtherActor)))
  (if (not (Variables|Default|GetIsConsumed))
    (if (Ability|HasAuthority)
      (bind _ascharacter (Utilities|Casting|CastToCharacter OtherActor))
      (bind _asbp_mogus_player_state (Utilities|Casting|CastToBP_MogusPlayerState (Variables|/Script/Engine.Controller|GetPlayerState (Pawn|GetController _ascharacter))))
      (if (Utilities|Enum|Equal(Enum) (Variables|/Game/Blueprints/Framework/BP_MogusPlayerState.BP_MogusPlayerState_C|GetPlayerAbility _asbp_mogus_player_state) "NewEnumerator0")
        (Default|ServerSetAbility _asbp_mogus_player_state (Variables|Default|GetAbility))
        (Variables|Default|SetIsConsumed true)
        (else
          (Development|PrintString (Utilities|String|Append (PlayerState|GetPlayerName _asbp_mogus_player_state) "! fuck off, you already have an ability")))))))

(event EventBeginPlay
  (bind _returnvalue (Rendering|Material|CreateDynamicMaterialInstance (Variables|Default|GetCube) 0 "/Game/LevelPrototyping/Materials/M_Color.M_Color" "None" :!class /Script/Engine.PrimitiveComponent))
  (Variables|Default|SetMaterial _returnvalue)
  (bind _returnvalue_2 (Utilities|GetDataTableRow "/Game/Blueprints/Framework/Abilities/DT_AbilityStats.DT_AbilityStats" (Utilities|String|StringToName (Utilities|String|EnumtoString (Variables|Default|GetAbility))))
    (:then
      (Rendering|Material|SetVectorParameterValue (Variables|Default|GetMaterial) "Color" (Math|Conversions|ToLinearColor(Color) (.Color (Utilities|Struct|BreakS_AbilityStats _returnvalue_2))) :!class /Script/Engine.MaterialInstanceDynamic))))

(event Collision|EventActorBeginOverlap
  (params (OtherActor :type Actor%20Object%20Reference)))

(fn ConstructionScript)

(fn OnRepIsConsumed
  (if (Variables|Default|GetIsConsumed)
    (Actor|DestroyActor)))